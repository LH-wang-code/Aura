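; Enemy summon ability that plays the shaman's summon montage and spawns random minions around the battlefield at points from GetActorSpawnLocation.
; On activation it shuffles those points and shows a Niagara ground effect at each.
; The montage's attack event starts a delayed loop that spawns one AI-possessed minion per point, facing the summoner.
; Each spawn increments the summoner's minion count through a message, and each minion's destruction decrements it.
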(event Custom|OnMinionDestroyed
  (params (DestroyedActor :type Actor%20Object%20Reference))
  (Class|CombatInterface|IncreaseMinionAmount(Message) (Ability|GetAvatarActorfromActorInfo) -1))

(event Ability|EventActivateAbility
  (bind _returnvalue (Class|AuraSummonAbility|GetActorSpawnLocation))
  (bind _output_get (Variables|Default|SetSpawnLocation _returnvalue))
  (Utilities|Array|Shuffle _output_get)
  (for _array_element (Variables|Default|GetSpawnLocation)
    (Niagara|SpawnSystematLocation "/Game/Assets/Effects/Combat/NS_GroundSummon.NS_GroundSummon" _array_element))
  (|PlayMontageandWaitProxy "None" "/Game/Assets/Enemies/Shaman/Animations/AM_Shaman_Summon.AM_Shaman_Summon" 1.0 "None" false 1.0 0.0 false
    (:then
      (Ability|Tasks|WaitGameplayEvent "(TagName=\"Montage.Attack.1\")" 0 true
        (:EventReceived
          (if (< (Variables|Default|GetSpawnLocationIndex) (Utilities|Array|Length (Variables|Default|GetSpawnLocation))) :!label _label
            (bind _returnvalue_2 (Class|AuraSummonAbility|GetRandomMinionClass))
            (bind _returnvalue_3 (Game|SpawnActorfromClass _returnvalue_2 (Math|Transform|MakeTransform (+ (Utilities|Array|Get(acopy) (Variables|Default|GetSpawnLocation) (Variables|Default|GetSpawnLocationIndex)) "0.000000,0.000000,70.000000") (Math|Rotator|FindLookatRotation (Utilities|Array|Get(acopy) (Variables|Default|GetSpawnLocation) (Variables|Default|GetSpawnLocationIndex)) (Transformation|GetActorLocation (Ability|GetAvatarActorfromActorInfo))) "1.000000,1.000000,1.000000") "AlwaysSpawn" "MultiplyWithRoot" 0 0))
            (Game|AssignOnDestroyed _returnvalue_3 (delegate Custom|OnMinionDestroyed))
            (Pawn|SpawnDefaultController _returnvalue_3)
            (Class|CombatInterface|IncreaseMinionAmount(Message) (Ability|GetAvatarActorfromActorInfo) 1)
            (Math|Integer|IncrementInt (Variables|Default|GetSpawnLocationIndex)
              (:%20%20
                (Utilities|FlowControl|Delay 0.2)
                (goto _label)))))))))

(event Ability|EventOnEndAbility
  (params (bWasCancelled :type Boolean)))