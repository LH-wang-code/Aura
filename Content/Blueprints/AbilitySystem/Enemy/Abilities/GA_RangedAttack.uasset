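; Enemy ranged attack gameplay ability that fires a projectile at the avatar's combat target.
; On activation it updates facing toward the target, then plays a random attack montage from the avatar's montage info.
; The montage's gameplay event spawns the projectile using the socket tag and the target's location at that moment.
; The ability ends when the montage completes or is interrupted or cancelled; debug-sphere and radius-damage nodes are left unconnected.
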(event Ability|EventActivateAbility
  (bind _returnvalue (Ability|GetAvatarActorfromActorInfo))
  (bind _returnvalue_2 (Ability|GetAvatarActorfromActorInfo))
  (bind _returnvalue_3 (Class|EnemyInterface|GetCombatTarget(Message) _returnvalue))
  (Class|CombatInterface|UpdateFacingTarget(Message) _returnvalue (Transformation|GetActorLocation _returnvalue_3))
  (bind _returnvalue_4 (Class|CombatInterface|GetAttackMontageTag(Message) (Ability|GetAvatarActorfromActorInfo)))
  (bind _output_get (Variables|Default|SetMontageInfo (Class|AuraDamageGameplayAbility|GetRandomMontagefromInfoArray _returnvalue_4)))
  (|PlayMontageandWaitProxy "None" (.AttackMontage (Utilities|Struct|BreakTaggedMontageInfo _output_get)) 1.0 "None" false 1.0 0.0 false
    (:then
      (Ability|Tasks|WaitGameplayEvent (.MontageTag (Utilities|Struct|BreakTaggedMontageInfo _output_get)) 0
        (:EventReceived
          (Class|CombatInterface|GetCombatSocketLocation(Message) _returnvalue_2 (.MontageTag (Utilities|Struct|BreakTaggedMontageInfo _output_get)))
          (bind _returnvalue_5 (Class|EnemyInterface|GetCombatTarget(Message) _returnvalue_2))
          (Class|AuraProjectileSpell|SpawnProjectile (Transformation|GetActorLocation _returnvalue_5) (.SocketTag (Utilities|Struct|BreakTaggedMontageInfo _output_get))))))
    (:OnCompleted
      (Ability|EndAbility :!label _label))
    (:OnInterrupted
      (goto _label))
    (:OnCancelled
      (goto _label))))

(event Ability|EventOnEndAbility
  (params (bWasCancelled :type Boolean)))