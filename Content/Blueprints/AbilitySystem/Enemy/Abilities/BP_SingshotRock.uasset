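; BP_SingshotRock is a rock actor for an enemy ability, apparently a slingshot projectile judging by its name, that tumbles visually.
; BeginPlay picks random yaw, pitch and roll rates, so each instance spins differently in either direction.
; Tick scales those rates by delta time and applies them as local rotation to the static mesh.
; The graph itself contains no movement, collision or damage logic.
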(event EventBeginPlay
  (bind _returnvalue (Math|Random|RandomFloatinRange -3.6e+02 3.6e+02))
  (Variables|Default|SetYawRotationRate _returnvalue)
  (Variables|Default|SetPitchRotationRate _returnvalue)
  (Variables|Default|SetRollRorationRate _returnvalue))

(event Collision|EventActorBeginOverlap
  (params (OtherActor :type Actor%20Object%20Reference)))

(event EventTick
  (params (DeltaSeconds :type Float%20%28single-precision%29))
  (Transformation|AddLocalRotation (Variables|Default|GetStaticMesh) (Math|Rotator|MakeRotator (* DeltaSeconds (Variables|Default|GetRollRorationRate)) (* DeltaSeconds (Variables|Default|GetPitchRotationRate)) (* DeltaSeconds (Variables|Default|GetYawRotationRate))) false false))

(fn ConstructionScript)