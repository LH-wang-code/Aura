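; Enemy melee attack gameplay ability that faces the combat target and plays a random attack montage from the avatar.
; At the montage's event tag, it damages living non-friend players in a small sphere around the montage's combat socket, spawning their blood effects.
; It then executes an impact GameplayCue, even on a miss because HasHit starts true, and ends.
; Montage completion, interruption or cancellation also ends the ability.
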(event Ability|EventActivateAbility
  (bind _returnvalue (Ability|GetAvatarActorfromActorInfo))
  (bind _returnvalue_2 (Ability|GetAvatarActorfromActorInfo))
  (bind _returnvalue_3 (Ability|GetAvatarActorfromActorInfo))
  (Variables|Default|SetHasHit true)
  ;[0.15 0.15 0.15 0.5] 跟随目标方向
  (bind _returnvalue_4 (Class|EnemyInterface|GetCombatTarget(Message) _returnvalue))
  (bind _ascombat_interface (Utilities|Casting|CastToCombatInterface _returnvalue))
  (Class|CombatInterface|UpdateFacingTarget _ascombat_interface (Transformation|GetActorLocation _returnvalue_4))
  (bind _returnvalue_5 (Class|CombatInterface|GetAttackMontageTag(Message) (Ability|GetAvatarActorfromActorInfo)))
  (bind _output_get (Variables|Default|SetMontageInfo (Class|AuraDamageGameplayAbility|GetRandomMontagefromInfoArray _returnvalue_5)))
  (|PlayMontageandWaitProxy "None" (.AttackMontage (Utilities|Struct|BreakTaggedMontageInfo _output_get)) 1.0 "None" false 1.0 0.0 false
    (:then
      (Ability|Tasks|WaitGameplayEvent (.MontageTag (Utilities|Struct|BreakTaggedMontageInfo _output_get)) 0
        (:EventReceived
          (bind _returnvalue_6 (Class|CombatInterface|GetCombatSocketLocation(Message) _returnvalue_3 (.SocketTag (Utilities|Struct|BreakTaggedMontageInfo _output_get))))
          (bind _outoverlappingactors (Class|AuraAbilitySystemFunctionLibrary|GetLivePlayersWithinRadius _returnvalue_3 (Utilities|Array|MakeArray _returnvalue_3) 45.0 _returnvalue_6))
          (for _array_element _outoverlappingactors
            (bind _returnvalue_7 (Class|AuraAbilitySystemFunctionLibrary|IsNotFriend (Ability|GetAvatarActorfromActorInfo) _array_element))
            (if _returnvalue_7
              (Class|AuraDamageGameplayAbility|CauseDamage _array_element)
              (Variables|Default|SetHasHit true)
              (bind _returnvalue_8 (Class|CombatInterface|GetBloodEffect(Message) _array_element))
              (Niagara|SpawnSystematLocation _returnvalue_8 _returnvalue_6)))
          (if (Variables|Default|GetHasHit)
            (bind _returnvalue_9 (Class|EnemyInterface|GetCombatTarget(Message) _returnvalue_2))
            (Class|GameplayAbility|ExecuteGameplayCuewithParams "(TagName=\"GameplayCue.ImpactEffect\")" (Ability|GameplayCue|MakeGameplayCueParameters :AggregatedTargetTags (GameplayTags|MakeGameplayTagContainerfromTag (.SocketTag (Utilities|Struct|BreakTaggedMontageInfo (Variables|Default|GetMontageInfo)))) :Location _returnvalue_6 :EffectCauser _returnvalue_2 :SourceObject _returnvalue_9)))
          (Ability|EndAbility))))
    (:OnCompleted
      (Ability|EndAbility :!label _label))
    (:OnInterrupted
      (goto _label))
    (:OnCancelled
      (goto _label))))

(event Ability|EventOnEndAbility
  (params (bWasCancelled :type Boolean)))