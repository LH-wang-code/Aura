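; BP_FramePillar is a pillar actor whose point light varies in intensity continuously during play.
; On BeginPlay it randomly picks one of two timelines, each of which drives the light with its own curve scaled by the FrameIntensity variable.
; When a timeline finishes, it picks again at random, producing an endless, irregular flicker without using Tick.
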(event Custom|StartTimeLine1
  (bind _frameintensity_1 (Timeline|Intensity_1 PlayFromStart)
    (:Update
      (Rendering|Components|Light|SetIntensity (Variables|Default|GetPointLight) (* _frameintensity_1 (Variables|Default|GetFrameIntensity))))
    (:Finished
      (CallFunction|ChooseIntensity))))

(event Custom|StartTimeLine2
  (bind _frameintensity_2 (Timeline|Intensity_2 PlayFromStart)
    (:Update
      (Rendering|Components|Light|SetIntensity (Variables|Default|GetPointLight) (* _frameintensity_2 (Variables|Default|GetFrameIntensity))))
    (:Finished
      (CallFunction|ChooseIntensity))))

(event Custom|ChooseIntensity
  (switch int (Math|Random|RandomIntegerinRange 0 1)
    (:0
      (CallFunction|StartTimeLine1))
    (:1
      (CallFunction|StartTimeLine2))))

(event EventBeginPlay
  (CallFunction|ChooseIntensity))

(event Collision|EventActorBeginOverlap
  (params (OtherActor :type Actor%20Object%20Reference)))

(event EventTick
  (params (DeltaSeconds :type Float%20%28single-precision%29)))

(fn ConstructionScript)