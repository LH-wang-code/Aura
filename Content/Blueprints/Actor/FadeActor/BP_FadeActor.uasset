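; Actor whose static mesh fades out and back in through the FadeOutInterface and FadeinInterface events, which play or reverse a timeline.
; Construction caches the original materials and builds dynamic instances from FadeMaterialInst, which are applied on BeginPlay and during fades.
; The timeline drives their "Fade" parameter.
; On finish, a value of 1 restores original materials and blocks GameTraceChannel2, while 0 makes the mesh ignore that channel.
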(event EventBeginPlay
  (CallFunction|SetDynamicMaterialInst))

(event EventFadeinInterface
  (bind _newtrack_0 (Timeline|Timeline Reverse)
    (:Update
      (CallFunction|SetDynamicMaterialsInstance)
      (for _array_element (Variables|Default|GetDynamicMaterialInst)
        (Rendering|Material|SetScalarParameterValue _array_element "Fade" _newtrack_0 :!class /Script/Engine.MaterialInstanceDynamic)))
    (:Finished
      (if (>= _newtrack_0 1.0)
        (CallFunction|ResetMaterials)
        (Collision|SetCollisionResponsetoChannel (Variables|Default|GetStaticMesh) "ECC_GameTraceChannel2" "ECR_Block")
        (elif (<= _newtrack_0 0.0)
          (Collision|SetCollisionResponsetoChannel (Variables|Default|GetStaticMesh) "ECC_GameTraceChannel2" "ECR_Ignore"))))))

(event EventFadeOutInterface
  (bind _newtrack_0 (Timeline|Timeline Play)
    (:Update
      (CallFunction|SetDynamicMaterialsInstance)
      (for _array_element (Variables|Default|GetDynamicMaterialInst)
        (Rendering|Material|SetScalarParameterValue _array_element "Fade" _newtrack_0 :!class /Script/Engine.MaterialInstanceDynamic)))
    (:Finished
      (if (>= _newtrack_0 1.0)
        (CallFunction|ResetMaterials)
        (Collision|SetCollisionResponsetoChannel (Variables|Default|GetStaticMesh) "ECC_GameTraceChannel2" "ECR_Block")
        (elif (<= _newtrack_0 0.0)
          (Collision|SetCollisionResponsetoChannel (Variables|Default|GetStaticMesh) "ECC_GameTraceChannel2" "ECR_Ignore"))))))

(fn ConstructionScript
  (Utilities|Array|Clear (Variables|Default|GetDynamicMaterialInst))
  (Variables|Default|SetOriginalMaterials (Rendering|Material|GetMaterials (Variables|Default|GetStaticMesh)))
  (for _array_element (Variables|Default|GetFadeMaterialInst)
    (bind _returnvalue (Rendering|Material|CreateDynamicMaterialInstance _array_element "None" "None" :!class /Script/Engine.KismetMaterialLibrary))
    (Utilities|Array|AddUnique (Variables|Default|GetDynamicMaterialInst) _returnvalue)))

(fn SetDynamicMaterialInst
  (for (_array_element _array_index) (Variables|Default|GetDynamicMaterialInst)
    (Rendering|Material|SetMaterial (Variables|Default|GetStaticMesh) _array_index _array_element)))

(fn ResetMaterials
  (for (_array_element _array_index) (Variables|Default|GetOriginalMaterials)
    (Rendering|Material|SetMaterial (Variables|Default|GetStaticMesh) _array_index _array_element)))

(fn SetDynamicMaterialsInstance
  (for (_array_element _array_index) (Variables|Default|GetDynamicMaterialInst)
    (Rendering|Material|SetMaterial (Variables|Default|GetStaticMesh) _array_index _array_element)))